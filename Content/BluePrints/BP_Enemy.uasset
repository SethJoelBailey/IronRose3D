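; BP_Enemy is an enemy pawn that chases the player and drops a coin when destroyed.
; PawnSensing sets IsSeeingPlayer on seeing any pawn, then FollowPlayer runs AIMoveTo toward player character 0; the flag is never cleared here.
; Any capsule hit, with no filter on the other actor, prints debug text, destroys the enemy and spawns BP_Coin 1000 units above its position.
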(event `self.ReceiveActorBeginOverlap`
  (params (OtherActor :type "Actor Object Reference")))

(event `self.CapsuleComponent.OnComponentHit`
  (params (HitComponent :type "PrimitiveComponent Object Reference") (OtherActor :type "Actor Object Reference") (OtherComp :type "PrimitiveComponent Object Reference") (NormalImpulse :type "Vector Structure") (Hit :type "HitResult Structure (by ref)"))
  (`KismetSystemLibrary.PrintText` "Hello")
  (`self.K2_DestroyActor`)
  (`|SpawnActorFromClass` "/Game/BluePrints/BP_Coin.BP_Coin_C" (`KismetMathLibrary.MakeTransform` (`KismetMathLibrary.MakeVector` (.x (.location (`self.GetTransform`))) (.y (.location (`self.GetTransform`))) (+ (.z (.location (`self.GetTransform`))) 1000.0))) "AdjustIfPossibleButAlwaysSpawn" "OverrideRootScale" null null))

(event `self.PawnSensing.OnSeePawn`
  (params (Pawn :type "Pawn Object Reference"))
  (set `self.IsSeeingPlayer?` true)
  (`self.FollowPlayer`))

(event `FollowPlayer`
  (if (`self.IsSeeingPlayer?`)
    (`|AIMoveTo` self (0.0 0.0 0.0) (`GameplayStatics.GetPlayerCharacter` 0))))

(fn `UserConstructionScript`)